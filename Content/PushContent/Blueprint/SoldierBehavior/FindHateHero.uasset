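; Behavior tree task that picks an enemy hero for a MOBA soldier to attack, judged by whether that hero is attacking an allied hero.
; It scans all hero actors for attackable other-camp heroes within a 2D search radius that pass the soldier's aggression check, keeping the nearest.
; The target is written to the HeroToAttack blackboard key, succeeding only if valid and attackable.
; MinDistance and TargetHero are not reset within the execute event.
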(event EventReceiveExecute
  (params (OwnerActor :type Actor%20Object%20Reference))
  (if (!= (Variables|Default|GetMOBASoldier_CON_Ref) 0)
    _
    (else
      (bind _asbp_mobasoldier_con (Utilities|Casting|CastToBP_MOBASoldier_Con OwnerActor))
      (Variables|Default|SetMOBASoldier_CON_Ref _asbp_mobasoldier_con)))
  (bind _asmobasoldier_character (Utilities|Casting|CastToMOBASoldierCharacter (Pawn|GetControlledPawn (Variables|Default|GetMOBASoldier_CON_Ref))))
  (bind _returnvalue (Class|MOBABaseCharacter|GetCamp _asmobasoldier_character))
  (Variables|Default|SetMyCamp _returnvalue)
  (Variables|Default|SetMyLocation (Transformation|GetActorLocation (Pawn|GetControlledPawn (Variables|Default|GetMOBASoldier_CON_Ref))))
  (bind _outactors (Actor|GetAllActorsOfClass "/Script/AMOBAProject.MOBAHeroCharacter"))
  (bind _output_get (Variables|Default|SetAllHero _outactors))
  (for _array_element _output_get
    (bind _returnvalue_2 (Class|MOBABaseCharacter|GetCamp _array_element))
    (bind _returnvalue_3 (Class|MOBABaseCharacter|GetbCanbeAttacked _array_element))
    (bind _returnvalue_4 (Class|MOBASoldierCharacter|IsEnemyHeroAttackingMyHero _asmobasoldier_character _array_element))
    (if (Math|Boolean|ANDBoolean (<= (Math|Vector|Distance2D(Vector) (Transformation|GetActorLocation _array_element) (Variables|Default|GetMyLocation)) (Variables|Default|GetSearchDistance)) (Utilities|Enum|NotEqual(Enum) _returnvalue_2 (Variables|Default|GetMyCamp)) _returnvalue_3 _returnvalue_4)
      (if (< (Math|Vector|Distance2D(Vector) (Transformation|GetActorLocation _array_element) (Variables|Default|GetMyLocation)) (Variables|Default|GetMinDistance))
        (Variables|Default|SetMinDistance (Math|Vector|Distance2D(Vector) (Transformation|GetActorLocation _array_element) (Variables|Default|GetMyLocation)))
        (Variables|Default|SetTargetHero _array_element))))
  (if (Utilities|IsValid (Variables|Default|GetTargetHero))
    (bind _returnvalue_5 (Class|MOBABaseCharacter|GetbCanbeAttacked (Variables|Default|GetTargetHero)))
    (if _returnvalue_5
      (Class|BTFunctionLibrary|SetBlackboardValueasObject (Variables|Default|GetHeroToAttack) (Variables|Default|GetTargetHero))
      (AI|BehaviorTree|FinishExecute true)
      (else
        (AI|BehaviorTree|FinishExecute false :!label _label)))
    (else
      (goto _label))))