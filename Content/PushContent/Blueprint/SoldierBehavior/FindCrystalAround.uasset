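; Behavior tree task for MOBA soldiers that finds the nearest enemy crystal to attack.
; On execute it caches the soldier controller, then scans every MOBABaseActor for attackable ones of another camp within a 2D search radius.
; It writes the closest to the CrystalToAttack blackboard key and reports success even if none qualifies.
; The running minimum distance and target are not reset between executions in this graph.
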(event EventReceiveExecute
  (params (OwnerActor :type Actor%20Object%20Reference))
  (if (!= (Variables|Default|GetMOBASoldier_CON_Ref) 0)
    _
    (else
      (bind _asbp_mobasoldier_con (Utilities|Casting|CastToBP_MOBASoldier_Con OwnerActor))
      (Variables|Default|SetMOBASoldier_CON_Ref _asbp_mobasoldier_con)))
  (bind _asmobabase_character (Utilities|Casting|CastToMOBABaseCharacter (Pawn|GetControlledPawn (Variables|Default|GetMOBASoldier_CON_Ref))))
  (bind _returnvalue (Class|MOBABaseCharacter|GetCamp _asmobabase_character))
  (Variables|Default|Setmycamp _returnvalue)
  (Variables|Default|SetMyLocation (Transformation|GetActorLocation (Pawn|GetControlledPawn (Variables|Default|GetMOBASoldier_CON_Ref))))
  (bind _outactors (Actor|GetAllActorsOfClass "/Script/AMOBAProject.MOBABaseActor"))
  (bind _output_get (Variables|Default|SetAllCrystal _outactors))
  (for _array_element _output_get
    (bind _returnvalue_2 (Class|MOBABaseActor|GetCamp _array_element))
    (bind _returnvalue_3 (Class|MOBABaseActor|GetbAbletoAttack _array_element))
    (if (Math|Boolean|ANDBoolean (<= (Math|Vector|Distance2D(Vector) (Transformation|GetActorLocation _array_element) (Variables|Default|GetMyLocation)) (Variables|Default|GetSearchDistance)) (Utilities|Enum|NotEqual(Enum) _returnvalue_2 (Variables|Default|Getmycamp)) _returnvalue_3)
      (if (< (Math|Vector|Distance2D(Vector) (Transformation|GetActorLocation _array_element) (Variables|Default|GetMyLocation)) (Variables|Default|GetMinDistance))
        (Variables|Default|SetMinDistance (Math|Vector|Distance2D(Vector) (Transformation|GetActorLocation _array_element) (Variables|Default|GetMyLocation)))
        (Variables|Default|SetTargetCrystal _array_element))))
  (Class|BTFunctionLibrary|SetBlackboardValueasObject (Variables|Default|GetCrystalToAttack) (Variables|Default|GetTargetCrystal))
  (AI|BehaviorTree|FinishExecute true))