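; Behavior Tree task that steers a MOBA soldier back toward its lane line.
; It caches the soldier controller, then issues an AI move to the pawn's closest point on a line built from Blackboard StartLocation, with TargetToGo as direction.
; Without waiting for arrival, it clears IsGoingBack if the 2D distance to that point is within BackDistance, then finishes successfully.
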(event EventReceiveExecute
  (params (OwnerActor :type Actor%20Object%20Reference))
  (if (!= (Variables|Default|GetMOBASoldier_CON_Ref) 0)
    _
    (else
      (bind _asbp_mobasoldier_con (Utilities|Casting|CastToBP_MOBASoldier_Con OwnerActor))
      (Variables|Default|SetMOBASoldier_CON_Ref _asbp_mobasoldier_con)))
  (AI|AIMoveTo (Pawn|GetControlledPawn (Variables|Default|GetMOBASoldier_CON_Ref)) (Math|Vector|FindClosestPointonLine (Transformation|GetActorLocation (Pawn|GetControlledPawn (Variables|Default|GetMOBASoldier_CON_Ref))) (Class|BTFunctionLibrary|GetBlackboardValueasVector (Variables|Default|GetStartLocation)) (Class|BTFunctionLibrary|GetBlackboardValueasVector (Variables|Default|GetTargetToGo))) 0 1.0 false
    (:then
      (if (<= (Math|Vector|Distance2D(Vector) (Math|Vector|FindClosestPointonLine (Transformation|GetActorLocation (Pawn|GetControlledPawn (Variables|Default|GetMOBASoldier_CON_Ref))) (Class|BTFunctionLibrary|GetBlackboardValueasVector (Variables|Default|GetStartLocation)) (Class|BTFunctionLibrary|GetBlackboardValueasVector (Variables|Default|GetTargetToGo))) (Transformation|GetActorLocation (Pawn|GetControlledPawn (Variables|Default|GetMOBASoldier_CON_Ref)))) (Variables|Default|GetBackDistance))
        (Class|BTFunctionLibrary|SetBlackboardValueasBool (Variables|Default|GetIsGoingBack) (not (<= (Math|Vector|Distance2D(Vector) (Math|Vector|FindClosestPointonLine (Transformation|GetActorLocation (Pawn|GetControlledPawn (Variables|Default|GetMOBASoldier_CON_Ref))) (Class|BTFunctionLibrary|GetBlackboardValueasVector (Variables|Default|GetStartLocation)) (Class|BTFunctionLibrary|GetBlackboardValueasVector (Variables|Default|GetTargetToGo))) (Transformation|GetActorLocation (Pawn|GetControlledPawn (Variables|Default|GetMOBASoldier_CON_Ref)))) (Variables|Default|GetBackDistance)))))
      (AI|BehaviorTree|FinishExecute true))))