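; AI controller for MOBA soldier minions that sends each one toward the opposing camp's corner.
; On BeginPlay it loads the soldier blackboard, reads the controlled pawn's camp and writes TargetToGo and StartLocation from two hardcoded map positions, swapped by camp.
; It then runs the soldier behavior tree, stopping early if the pawn is not a MOBA soldier.
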(event EventBeginPlay
  (bind _self self)
  (bind _self_2 self)
  (bind _returnvalue (AI|GetBlackboard _self))
  (bind _returnvalue_2 (AI|GetBlackboard _self_2))
  (Class|AIController|UseBlackboard "/Game/PushContent/Blueprint/SoldierBehavior/BB_MOBASoldierCharacter.BB_MOBASoldierCharacter")
  (bind _asmobasoldier_character (Utilities|Casting|CastToMOBASoldierCharacter (Pawn|GetControlledPawn self)))
  (bind _returnvalue_3 (Class|MOBABaseCharacter|GetCamp _asmobasoldier_character))
  (bind _output_get (Variables|Default|SetBlueLocation "-8400.000000,-8400.000000,300.000000"))
  (bind _output_get_2 (Variables|Default|SetRedLocation "8400.000000,8400.000000,300.000000"))
  (if (Utilities|Enum|Equal(Enum) _returnvalue_3 "blue")
    (AI|Components|Blackboard|SetValueasVector _returnvalue_2 (Variables|Default|GetTargetToGo) _output_get_2)
    (AI|Components|Blackboard|SetValueasVector _returnvalue_2 (Variables|Default|GetStartLocation) _output_get)
    (AI|RunBehaviorTree "/Game/PushContent/Blueprint/SoldierBehavior/BT_MOBASoliderCharacter.BT_MOBASoliderCharacter")
    (else
      (AI|Components|Blackboard|SetValueasVector _returnvalue (Variables|Default|GetTargetToGo) _output_get)
      (AI|Components|Blackboard|SetValueasVector _returnvalue (Variables|Default|GetStartLocation) _output_get_2)
      (AI|RunBehaviorTree "/Game/PushContent/Blueprint/SoldierBehavior/BT_MOBASoliderCharacter.BT_MOBASoliderCharacter"))))

(fn ConstructionScript)