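; Behavior tree task that initializes a MOBA soldier's lane route.
; It caches the soldier AI controller, then uses the pawn's camp and road to write start and target locations to the blackboard.
; It sets the Init flag, orders a move to the closest point on the line through those locations, and finishes successfully without waiting for arrival.
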(event EventReceiveExecute
  (params (OwnerActor :type Actor%20Object%20Reference))
  (if (!= (Variables|Default|GetMOBASoldier_CON_Ref) 0)
    _
    (else
      (bind _asbp_mobasoldier_con (Utilities|Casting|CastToBP_MOBASoldier_Con OwnerActor))
      (Variables|Default|SetMOBASoldier_CON_Ref _asbp_mobasoldier_con)))
  (bind _asmobabase_character (Utilities|Casting|CastToMOBABaseCharacter (Pawn|GetControlledPawn (Variables|Default|GetMOBASoldier_CON_Ref))))
  (bind _returnvalue (Class|MOBABaseCharacter|GetCamp _asmobabase_character))
  (if (Utilities|Enum|Equal(Enum) _returnvalue "blue")
    (bind _asmobasoldier_character (Utilities|Casting|CastToMOBASoldierCharacter (Pawn|GetControlledPawn (Variables|Default|GetMOBASoldier_CON_Ref))))
    (bind _returnvalue_2 (Class|MOBASoldierCharacter|GetRoad _asmobasoldier_character))
    (switch Utilities|FlowControl|Switch|SwitchonSoldierRoad _returnvalue_2
      (:soldierTop
        (AI|BehaviorTree|SetBlackboardValueasVector (Variables|Default|GetTargetToGo) (Variables|Default|GetNorthWestLocation))
        (AI|BehaviorTree|SetBlackboardValueasVector (Variables|Default|GetStartLocation) (Variables|Default|GetBlueLocation)))
      (:soldierMid
        (AI|BehaviorTree|SetBlackboardValueasVector (Variables|Default|GetTargetToGo) (Variables|Default|GetRedLocation))
        (AI|BehaviorTree|SetBlackboardValueasVector (Variables|Default|GetStartLocation) (Variables|Default|GetBlueLocation)))
      (:soldierDown
        (AI|BehaviorTree|SetBlackboardValueasVector (Variables|Default|GetTargetToGo) (Variables|Default|GetSouthEastLocation))
        (AI|BehaviorTree|SetBlackboardValueasVector (Variables|Default|GetStartLocation) (Variables|Default|GetBlueLocation))))
    (else
      (bind _asmobasoldier_character_2 (Utilities|Casting|CastToMOBASoldierCharacter (Pawn|GetControlledPawn (Variables|Default|GetMOBASoldier_CON_Ref))))
      (bind _returnvalue_3 (Class|MOBASoldierCharacter|GetRoad _asmobasoldier_character_2))
      (switch Utilities|FlowControl|Switch|SwitchonSoldierRoad _returnvalue_3
        (:soldierTop
          (AI|BehaviorTree|SetBlackboardValueasVector (Variables|Default|GetTargetToGo) (Variables|Default|GetSouthEastLocation))
          (AI|BehaviorTree|SetBlackboardValueasVector (Variables|Default|GetStartLocation) (Variables|Default|GetRedLocation)))
        (:soldierMid
          (AI|BehaviorTree|SetBlackboardValueasVector (Variables|Default|GetTargetToGo) (Variables|Default|GetBlueLocation))
          (AI|BehaviorTree|SetBlackboardValueasVector (Variables|Default|GetStartLocation) (Variables|Default|GetRedLocation)))
        (:soldierDown
          (AI|BehaviorTree|SetBlackboardValueasVector (Variables|Default|GetTargetToGo) (Variables|Default|GetNorthWestLocation))
          (AI|BehaviorTree|SetBlackboardValueasVector (Variables|Default|GetStartLocation) (Variables|Default|GetRedLocation))))))
  (Class|BTFunctionLibrary|SetBlackboardValueasBool (Variables|Default|GetInit) true)
  (AI|Navigation|MovetoLocation (Variables|Default|GetMOBASoldier_CON_Ref) (Math|Vector|FindClosestPointonLine (Transformation|GetActorLocation (Pawn|GetControlledPawn (Variables|Default|GetMOBASoldier_CON_Ref))) (Class|BTFunctionLibrary|GetBlackboardValueasVector (Variables|Default|GetStartLocation)) (- (Class|BTFunctionLibrary|GetBlackboardValueasVector (Variables|Default|GetStartLocation)) (Class|BTFunctionLibrary|GetBlackboardValueasVector (Variables|Default|GetTargetToGo)))) 0.1 true true false true 0)
  (AI|BehaviorTree|FinishExecute true))