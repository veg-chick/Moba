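; Behavior tree task that sends a MOBA soldier toward the enemy or assigned tower stored in its TargetTower blackboard key.
; It caches the soldier AI controller on first execution, then calls MoveToLocation on the tower's position, using the pawn's attack range as acceptance radius.
; It finishes successfully right after issuing the move, without waiting for arrival, and fails when no valid target exists.
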(event EventReceiveExecute
  (params (OwnerActor :type Actor%20Object%20Reference))
  (bind _targettower (Variables|Default|GetTargetTower))
  (bind _returnvalue (Class|BTFunctionLibrary|GetBlackboardValueasObject _targettower))
  (if (!= (Variables|Default|GetMOBASoldier_CON_Ref) 0)
    _
    (else
      (bind _asbp_mobasoldier_con (Utilities|Casting|CastToBP_MOBASoldier_Con OwnerActor))
      (Variables|Default|SetMOBASoldier_CON_Ref _asbp_mobasoldier_con)))
  (if (Utilities|IsValid _returnvalue)
    (bind _asmobatower_character (Utilities|Casting|CastToMOBATowerCharacter _returnvalue))
    (bind _asmobasoldier_character (Utilities|Casting|CastToMOBASoldierCharacter (Pawn|GetControlledPawn (Variables|Default|GetMOBASoldier_CON_Ref))))
    (bind _returnvalue_2 (Class|MOBABaseCharacter|GetAttackRange _asmobasoldier_character))
    (AI|Navigation|MovetoLocation (Variables|Default|GetMOBASoldier_CON_Ref) (Transformation|GetActorLocation _asmobatower_character) _returnvalue_2 true true false true 0)
    (AI|BehaviorTree|FinishExecute true)
    (else
      (AI|BehaviorTree|FinishExecute false))))