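; Behavior tree task that makes a MOBA soldier attack its target tower.
; It caches the soldier's AI controller and reads the TargetTower blackboard object as a base character.
; If the tower is within the soldier's attack range in 2D distance, it triggers a single attack and finishes successfully.
; An invalid or out-of-range target fails the task.
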(event EventReceiveExecute
  (params (OwnerActor :type Actor%20Object%20Reference))
  (bind _targettower (Variables|Default|GetTargetTower))
  (bind _returnvalue (Class|BTFunctionLibrary|GetBlackboardValueasObject _targettower))
  (if (!= (Variables|Default|GetMOBASoldier_CON_Ref) 0)
    _
    (else
      (bind _asbp_mobasoldier_con (Utilities|Casting|CastToBP_MOBASoldier_Con OwnerActor))
      (bind _output_get (Variables|Default|SetMOBASoldier_CON_Ref _asbp_mobasoldier_con))))
  (if (Utilities|IsValid _returnvalue)
    (bind _asmobabase_character (Utilities|Casting|CastToMOBABaseCharacter _returnvalue))
    (bind _asmobasoldier_character (Utilities|Casting|CastToMOBASoldierCharacter (Pawn|GetControlledPawn _output_get)))
    (bind _returnvalue_2 (Class|MOBABaseCharacter|GetAttackRange _asmobasoldier_character))
    (if (<= (Math|Vector|Distance2D(Vector) (Transformation|GetActorLocation _asmobabase_character) (Transformation|GetActorLocation _asmobasoldier_character)) _returnvalue_2)
      (Class|MOBASoldierCharacter|AttacktoCharacterOnce _asmobasoldier_character _asmobabase_character)
      (AI|BehaviorTree|FinishExecute true)
      (else
        (AI|BehaviorTree|FinishExecute false :!label _label)))
    (else
      (goto _label))))