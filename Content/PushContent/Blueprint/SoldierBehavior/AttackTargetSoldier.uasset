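; Behavior tree task that makes a MOBA soldier (minion) attack the character stored in its TargetSoldier blackboard key.
; It caches the soldier controller, then checks 2D distance against attack range plus both capsule radii.
; In range, it turns the soldier to face the target, triggers one attack and succeeds; out of range it fails.
; A failed cast exits without finishing the task.
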(event EventReceiveExecute
  (params (OwnerActor :type Actor%20Object%20Reference))
  (if (!= (Variables|Default|GetMOBASoldier_CON_Ref) 0)
    _
    (else
      (bind _asbp_mobasoldier_con (Utilities|Casting|CastToBP_MOBASoldier_Con OwnerActor))
      (bind _output_get (Variables|Default|SetMOBASoldier_CON_Ref _asbp_mobasoldier_con))))
  ;[1 1 1] 目标小兵 类型：BP MOBASoldier Character
  (bind _asmobabase_character (Utilities|Casting|CastToMOBABaseCharacter (Class|BTFunctionLibrary|GetBlackboardValueasObject (Variables|Default|GetTargetSoldier))))
  ;[1 1 1] 该小兵 类型：BP MOBASoldier Character
  (bind _asmobasoldier_character (Utilities|Casting|CastToMOBASoldierCharacter (Pawn|GetControlledPawn _output_get)))
  (bind _returnvalue (Class|MOBABaseCharacter|GetAttackRange _asmobasoldier_character))
  (if (<= (Math|Vector|Distance2D(Vector) (Transformation|GetActorLocation _asmobabase_character) (Transformation|GetActorLocation _asmobasoldier_character)) (+ (Components|Capsule|GetScaledCapsuleRadius (Variables|/Script/Engine.Character|GetCapsuleComponent _asmobabase_character)) _returnvalue (Components|Capsule|GetScaledCapsuleRadius (Variables|/Script/Engine.Character|GetCapsuleComponent _asmobasoldier_character))))
    (Transformation|SetActorRotation _asmobasoldier_character (Math|Conversions|RotationFromXVector (Math|Vector|Normalize (- (Transformation|GetActorLocation _asmobabase_character) (Transformation|GetActorLocation _asmobasoldier_character)))))
    (Class|MOBASoldierCharacter|AttacktoCharacterOnce _asmobasoldier_character _asmobabase_character)
    (AI|BehaviorTree|FinishExecute true)
    (else
      (AI|BehaviorTree|FinishExecute false))))