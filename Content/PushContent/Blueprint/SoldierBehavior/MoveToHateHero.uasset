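; Behavior tree task that sends a MOBA soldier toward the hero stored in the TargetHero blackboard key.
; It caches the soldier's AI controller, then calls MoveToLocation on the hero's current position, using the soldier's attack range as acceptance radius.
; It finishes successfully right after issuing the move, without waiting for arrival, and fails when no valid target is set.
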(event EventReceiveExecute
  (params (OwnerActor :type Actor%20Object%20Reference))
  (bind _targethero (Variables|Default|GetTargetHero))
  (bind _returnvalue (Class|BTFunctionLibrary|GetBlackboardValueasObject _targethero))
  (if (!= (Variables|Default|GetMOBASoldier_CON_Ref) 0)
    _
    (else
      (bind _asbp_mobasoldier_con (Utilities|Casting|CastToBP_MOBASoldier_Con OwnerActor))
      (bind _output_get (Variables|Default|SetMOBASoldier_CON_Ref _asbp_mobasoldier_con))))
  (bind _asmobasoldier_character (Utilities|Casting|CastToMOBASoldierCharacter (Pawn|GetControlledPawn _output_get)))
  (if (Utilities|IsValid _returnvalue)
    (bind _asmobahero_character (Utilities|Casting|CastToMOBAHeroCharacter _returnvalue))
    (bind _returnvalue_2 (Class|MOBABaseCharacter|GetAttackRange _asmobasoldier_character))
    (AI|Navigation|MovetoLocation (Variables|Default|GetMOBASoldier_CON_Ref) (Transformation|GetActorLocation _asmobahero_character) _returnvalue_2 true true false true 0)
    (AI|BehaviorTree|FinishExecute true)
    (else
      (AI|BehaviorTree|FinishExecute false))))