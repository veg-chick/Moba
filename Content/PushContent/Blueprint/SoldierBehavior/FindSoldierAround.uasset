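; Behavior tree task that finds the nearest attackable enemy soldier for a MOBA soldier AI.
; On tick it scans all MOBASoldierCharacter actors, filtering by opposing camp, attackable flag and 2D distance within AttackDistance.
; The closest match under MinDistance is written to the SoldierToAttack blackboard key, then the task finishes successfully.
; The graph never resets MinDistance or TargetSoldier before scanning.
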(event EventTick
  (params (OwnerActor :type Actor%20Object%20Reference) (DeltaSeconds :type Float%20%28single-precision%29))
  (bind _asbp_mobasoldier_con (Utilities|Casting|CastToBP_MOBASoldier_Con (AI|GetAIController OwnerActor)))
  (Variables|Default|SetMOBASoldier_CON_Ref _asbp_mobasoldier_con)
  (bind _asmobasoldier_character (Utilities|Casting|CastToMOBASoldierCharacter (Pawn|GetControlledPawn (Variables|Default|GetMOBASoldier_CON_Ref))))
  (bind _returnvalue (Class|MOBABaseCharacter|GetCamp _asmobasoldier_character))
  (Variables|Default|SetMyCamp _returnvalue)
  (Variables|Default|SetMyLocation (Transformation|GetActorLocation (Pawn|GetControlledPawn (Variables|Default|GetMOBASoldier_CON_Ref))))
  (bind _outactors (Actor|GetAllActorsOfClass "/Script/AMOBAProject.MOBASoldierCharacter"))
  (bind _output_get (Variables|Default|SetAllsoldiers _outactors))
  (for _array_element _output_get
    (bind _returnvalue_2 (Class|MOBABaseCharacter|GetCamp _array_element))
    (bind _returnvalue_3 (Class|MOBABaseCharacter|GetbCanbeAttacked _array_element))
    (if (Math|Boolean|ANDBoolean (<= (Math|Vector|Distance2D(Vector) (Transformation|GetActorLocation _array_element) (Variables|Default|GetMyLocation)) (Variables|Default|GetAttackDistance)) (Utilities|Enum|NotEqual(Enum) (Variables|Default|GetMyCamp) _returnvalue_2) (!= (Math|Vector|Distance2D(Vector) (Transformation|GetActorLocation _array_element) (Variables|Default|GetMyLocation)) 0.0) _returnvalue_3)
      (if (< (Math|Vector|Distance2D(Vector) (Transformation|GetActorLocation _array_element) (Variables|Default|GetMyLocation)) (Variables|Default|GetMinDistance))
        (Variables|Default|SetMinDistance (Math|Vector|Distance2D(Vector) (Transformation|GetActorLocation _array_element) (Variables|Default|GetMyLocation)))
        (Variables|Default|SetTargetSoldier _array_element))))
  (Class|BTFunctionLibrary|SetBlackboardValueasObject (Variables|Default|GetSoldierToAttack) (Variables|Default|GetTargetSoldier))
  (AI|BehaviorTree|FinishExecute true))