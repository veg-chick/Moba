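; Behavior tree tick node for MOBA soldiers that checks lane deviation and advances waypoints.
; Each tick it sets IsGoingBack when the pawn's distance from a line exceeds MaxDistance, passing StartLocation as origin and the TargetToGo position itself as direction.
; Within one unit of TargetToGo in 2D, it retargets Top and Down soldiers to the opposing camp's location, with a corner StartLocation chosen by camp and road.
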(event EventTick
  (params (OwnerActor :type Actor%20Object%20Reference) (DeltaSeconds :type Float%20%28single-precision%29))
  (if (!= (Variables|Default|GetMOBASoldier_CON_Ref) 0)
    _
    (else
      (bind _asbp_mobasoldier_con (Utilities|Casting|CastToBP_MOBASoldier_Con OwnerActor))
      (Variables|Default|SetMOBASoldier_CON_Ref _asbp_mobasoldier_con)))
  (Class|BTFunctionLibrary|SetBlackboardValueasBool (Variables|Default|GetIsGoingBack) (> (Math|Vector|GetPointDistancetoLine (Transformation|GetActorLocation (Pawn|GetControlledPawn (Variables|Default|GetMOBASoldier_CON_Ref))) (Class|BTFunctionLibrary|GetBlackboardValueasVector (Variables|Default|GetStartLocation)) (Class|BTFunctionLibrary|GetBlackboardValueasVector (Variables|Default|GetTargetToGo))) (Variables|Default|GetMaxDistance)))
  (if (<= (Math|Vector|Distance2D(Vector) (Class|BTFunctionLibrary|GetBlackboardValueasVector (Variables|Default|GetTargetToGo)) (Transformation|GetActorLocation (Pawn|GetControlledPawn (Variables|Default|GetMOBASoldier_CON_Ref)))) 1.0)
    (bind _asmobasoldier_character (Utilities|Casting|CastToMOBASoldierCharacter (Pawn|GetControlledPawn (Variables|Default|GetMOBASoldier_CON_Ref))))
    (bind _returnvalue (Class|MOBABaseCharacter|GetCamp _asmobasoldier_character))
    (switch Utilities|FlowControl|Switch|SwitchonCamp _returnvalue
      (:blue
        (bind _returnvalue_2 (Class|MOBASoldierCharacter|GetRoad _asmobasoldier_character))
        (switch Utilities|FlowControl|Switch|SwitchonSoldierRoad _returnvalue_2
          (:soldierTop
            (AI|BehaviorTree|SetBlackboardValueasVector (Variables|Default|GetTargetToGo) (Variables|Default|GetRedLocation))
            (AI|BehaviorTree|SetBlackboardValueasVector (Variables|Default|GetStartLocation) (Variables|Default|GetNorthWestLocation)))
          (:soldierDown
            (AI|BehaviorTree|SetBlackboardValueasVector (Variables|Default|GetTargetToGo) (Variables|Default|GetRedLocation))
            (AI|BehaviorTree|SetBlackboardValueasVector (Variables|Default|GetStartLocation) (Variables|Default|GetSouthEastLocation)))))
      (:red
        (bind _returnvalue_3 (Class|MOBASoldierCharacter|GetRoad _asmobasoldier_character))
        (switch Utilities|FlowControl|Switch|SwitchonSoldierRoad _returnvalue_3
          (:soldierTop
            (AI|BehaviorTree|SetBlackboardValueasVector (Variables|Default|GetTargetToGo) (Variables|Default|GetBlueLocation))
            (AI|BehaviorTree|SetBlackboardValueasVector (Variables|Default|GetStartLocation) (Variables|Default|GetSouthEastLocation)))
          (:soldierDown
            (AI|BehaviorTree|SetBlackboardValueasVector (Variables|Default|GetTargetToGo) (Variables|Default|GetBlueLocation))
            (AI|BehaviorTree|SetBlackboardValueasVector (Variables|Default|GetStartLocation) (Variables|Default|GetNorthWestLocation))))))))