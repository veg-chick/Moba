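; Behavior tree task that sends a MOBA soldier toward the hero stored in the TargetHero blackboard key.
; It caches the soldier AI controller, then checks the 2D distance from its pawn to the hero against MaxDistance.
; In range, it issues MoveToLocation with attack range as acceptance radius and succeeds immediately without awaiting arrival.
; Out of range it clears TargetHero and fails, as it does when no valid target exists.
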(event EventReceiveExecute
  (params (OwnerActor :type Actor%20Object%20Reference))
  (bind _targethero (Variables|Default|GetTargetHero))
  (bind _returnvalue (Class|BTFunctionLibrary|GetBlackboardValueasObject _targethero))
  (if (!= (Variables|Default|GetMOBASoldier_CON_Ref) 0)
    _
    (else
      (bind _asbp_mobasoldier_con (Utilities|Casting|CastToBP_MOBASoldier_Con OwnerActor))
      (Variables|Default|SetMOBASoldier_CON_Ref _asbp_mobasoldier_con)))
  (if (Utilities|IsValid _returnvalue)
    (bind _asbp_mobahero_character (Utilities|Casting|CastToBP_MOBAHeroCharacter _returnvalue))
    (if (<= (Math|Vector|Distance2D(Vector) (Transformation|GetActorLocation _asbp_mobahero_character) (Transformation|GetActorLocation (Pawn|GetControlledPawn (Variables|Default|GetMOBASoldier_CON_Ref)))) (Variables|Default|GetMax_Distance))
      (bind _asmobasoldier_character (Utilities|Casting|CastToMOBASoldierCharacter (Pawn|GetControlledPawn (Variables|Default|GetMOBASoldier_CON_Ref))))
      (bind _returnvalue_2 (Class|MOBABaseCharacter|GetAttackRange _asmobasoldier_character))
      (AI|Navigation|MovetoLocation (Variables|Default|GetMOBASoldier_CON_Ref) (Transformation|GetActorLocation _asbp_mobahero_character) _returnvalue_2 true true false true 0)
      (AI|BehaviorTree|FinishExecute true)
      (else
        (Class|BTFunctionLibrary|SetBlackboardValueasObject (Variables|Default|GetTargetHero))
        (AI|BehaviorTree|FinishExecute false :!label _label)))
    (else
      (goto _label))))