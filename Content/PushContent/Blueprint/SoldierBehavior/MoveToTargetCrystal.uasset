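; Behavior tree task that sends a MOBA soldier toward the crystal stored under its TargetCrystal blackboard key.
; It caches the soldier AI controller on first run, then calls MoveToActor using the controlled soldier's attack range as acceptance radius.
; It finishes successfully as soon as the move is issued, without waiting for arrival, and fails when no valid crystal is set.
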(event EventReceiveExecute
  (params (OwnerActor :type Actor%20Object%20Reference))
  (bind _targetcrystal (Variables|Default|GetTargetCrystal))
  (bind _returnvalue (Class|BTFunctionLibrary|GetBlackboardValueasObject _targetcrystal))
  (if (!= (Variables|Default|GetMOBASoldier_CON_Ref) 0)
    _
    (else
      (bind _asbp_mobasoldier_con (Utilities|Casting|CastToBP_MOBASoldier_Con OwnerActor))
      (Variables|Default|SetMOBASoldier_CON_Ref _asbp_mobasoldier_con)))
  (if (Utilities|IsValid _returnvalue)
    (bind _asmobabase_actor (Utilities|Casting|CastToMOBABaseActor _returnvalue))
    (bind _asmobasoldier_character (Utilities|Casting|CastToMOBASoldierCharacter (Pawn|GetControlledPawn (Variables|Default|GetMOBASoldier_CON_Ref))))
    (bind _returnvalue_2 (Class|MOBABaseCharacter|GetAttackRange _asmobasoldier_character))
    (AI|Navigation|MovetoActor (Variables|Default|GetMOBASoldier_CON_Ref) _asmobabase_actor _returnvalue_2 true true true 0)
    (AI|BehaviorTree|FinishExecute true)
    (else
      (AI|BehaviorTree|FinishExecute false))))