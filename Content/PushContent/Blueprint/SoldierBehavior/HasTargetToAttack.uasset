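; Behavior tree decorator for soldier AI that checks whether the soldier has anything to attack.
; It reads four blackboard object keys for hero, soldier, tower and crystal targets.
; The condition passes when at least one of those targets is valid, with no priority or distance logic.
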(fn PerformConditionCheck
  (params (OwnerActor :type Actor%20Object%20Reference))
  (return (Math|Boolean|ORBoolean (Utilities|IsValid (Class|BTFunctionLibrary|GetBlackboardValueasObject (Variables|Default|GetTargetHero))) (Utilities|IsValid (Class|BTFunctionLibrary|GetBlackboardValueasObject (Variables|Default|GetTargetSoldier))) (Utilities|IsValid (Class|BTFunctionLibrary|GetBlackboardValueasObject (Variables|Default|GetTargetTower))) (Utilities|IsValid (Class|BTFunctionLibrary|GetBlackboardValueasObject (Variables|Default|GetTargetCrystal))))))