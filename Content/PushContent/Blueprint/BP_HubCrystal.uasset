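; BP_HubCrystal is a MOBA hub crystal with a camp and hit points, shown through a HubCrystalUI widget component.
; On Tick, when player controller 0 is local, it pushes the Hp / MaxHp ratio into the widget.
; The same Tick colors the widget green for the local character's camp or red otherwise, latching with IsSet once a MOBABaseCharacter pawn is available.
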(event EventBeginPlay)

(event EventTick
  (params (DeltaSeconds :type Float%20%28single-precision%29))
  (bind _returnvalue (Game|GetPlayerController 0))
  (bind _ashub_crystal_ui (Utilities|Casting|CastToHubCrystalUI (UserInterface|GetUserWidgetObject (Variables|Default|GetWidget))))
  (Utilities|IsValid _returnvalue
    (:Is%20Valid
      (if (Pawn|IsLocalPlayerController _returnvalue)
        (Utilities|FlowControl|Sequence
          (:then_0
            (bind _returnvalue_2 (Class|MOBABaseActor|GetHp))
            (bind _returnvalue_3 (Class|MOBABaseActor|GetMaxHp))
            (Variables|/Game/PushContent/HUD/MOBAUI/HubCrystalUI.HubCrystalUI_C|SetHp _ashub_crystal_ui (/ _returnvalue_2 _returnvalue_3)))
          (:then_1
            (if (not (Variables|Default|GetIsSet))
              (bind _asmobabase_character (Utilities|Casting|CastToMOBABaseCharacter (Pawn|GetControlledPawn _returnvalue)))
              (bind _returnvalue_4 (Class|MOBABaseActor|GetCamp))
              (bind _returnvalue_5 (Class|MOBABaseCharacter|GetCamp _asmobabase_character))
              (if (Utilities|Enum|Equal(Enum) _returnvalue_5 _returnvalue_4)
                (Variables|/Game/PushContent/HUD/MOBAUI/HubCrystalUI.HubCrystalUI_C|SetColor _ashub_crystal_ui (Variables|Default|GetGreen))
                (else
                  (Variables|/Game/PushContent/HUD/MOBAUI/HubCrystalUI.HubCrystalUI_C|SetColor _ashub_crystal_ui (Variables|Default|GetRed))))
              (Variables|Default|SetIsSet true))))))))

(fn ConstructionScript)