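; MOBA hero character (Tank One) that assigns its team and drives its own hero state widget.
; On BeginPlay, a player-controlled hero maps its match player index to a camp: 0 is Red, 1 is Blue.
; Every Tick it pushes health and mana ratios and level into HeroStateUI, coloring health green when sharing the local player's camp and red otherwise.
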(event EventBeginPlay
  (bind _asplayer_controller (Utilities|Casting|CastToPlayerController (Pawn|GetController)))
  (bind _playerindex (Class|TurnBasedBlueprintLibrary|GetMyPlayerIndex _asplayer_controller _asplayer_controller))
  (switch int _playerindex
    (:0
      (Class|MOBABaseCharacter|SetCamp "red"))
    (:1
      (Class|MOBABaseCharacter|SetCamp "blue"))))

(event Collision|EventActorBeginOverlap
  (params (OtherActor :type Actor%20Object%20Reference)))

(event EventTick
  (params (DeltaSeconds :type Float%20%28single-precision%29))
  (Utilities|FlowControl|Sequence
    (:then_0
      (bind _ashero_state_ui (Utilities|Casting|CastToHeroStateUI (UserInterface|GetUserWidgetObject (Variables|Default|GetWidget))))
      (bind _returnvalue (Class|MOBABaseCharacter|GetHp))
      (bind _returnvalue_2 (Class|MOBABaseCharacter|GetMaxHp))
      (Variables|/Game/PushContent/HUD/MOBAUI/HeroStateUI.HeroStateUI_C|SetHealth _ashero_state_ui (/ _returnvalue _returnvalue_2))
      (bind _returnvalue_3 (Class|MOBABaseCharacter|GetCamp))
      (bind _asmobabase_character (Utilities|Casting|CastToMOBABaseCharacter (Game|GetPlayerCharacter 0)))
      (bind _returnvalue_4 (Class|MOBABaseCharacter|GetCamp _asmobabase_character))
      (if (Utilities|Enum|Equal(Enum) _returnvalue_3 _returnvalue_4)
        (Variables|/Game/PushContent/HUD/MOBAUI/HeroStateUI.HeroStateUI_C|SetHpColor _ashero_state_ui (Variables|Default|GetGreen))
        (else
          (Variables|/Game/PushContent/HUD/MOBAUI/HeroStateUI.HeroStateUI_C|SetHpColor _ashero_state_ui (Variables|Default|GetRed)))))
    (:then_1
      (bind _returnvalue_5 (Class|MOBABaseCharacter|GetMp))
      (bind _returnvalue_6 (Class|MOBABaseCharacter|GetMaxMp))
      (Variables|/Game/PushContent/HUD/MOBAUI/HeroStateUI.HeroStateUI_C|SetPower _ashero_state_ui (/ _returnvalue_5 _returnvalue_6)))
    (:then_2
      (bind _returnvalue_7 (Class|MOBABaseCharacter|GetLevel))
      (Variables|/Game/PushContent/HUD/MOBAUI/HeroStateUI.HeroStateUI_C|SetLv _ashero_state_ui (Utilities|Text|ToText(Float) _returnvalue_7 "HalfToEven" false true 1 324 0 0)))))

(fn ConstructionScript)