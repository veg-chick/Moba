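; BP_Wild is a placeholder actor that respawns MOBA wild monsters: Blue Buff, Red Buff or the Nash dragon.
; On WildResetHandle it branches on its wild type and spawns the matching AI pawn at its own transform with the shared BT_MOBAWildCharacter behavior tree.
; After a matching spawn the actor destroys itself; other types do nothing.
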(event EventBeginPlay)

(event Collision|EventActorBeginOverlap
  (params (OtherActor :type Actor%20Object%20Reference)))

(event EventTick
  (params (DeltaSeconds :type Float%20%28single-precision%29)))

(event EventWildResetHandle
  (bind _returnvalue (Transformation|GetActorLocation))
  (bind _returnvalue_2 (Transformation|GetActorRotation))
  (bind _returnvalue_3 (Class|MOBAWildCharacter|GetWildType))
  (if (Utilities|Enum|Equal(Enum) _returnvalue_3 "BlueBuff")
    (AI|SpawnAIFromClass "/Game/PushContent/Blueprint/BP_BlueBuff.BP_BlueBuff_C" "/Game/PushContent/Blueprint/WildBehavior/BT_MOBAWildCharacter.BT_MOBAWildCharacter" _returnvalue _returnvalue_2 false)
    (Actor|DestroyActor)
    (elif (Utilities|Enum|Equal(Enum) _returnvalue_3 "RedBuff")
      (AI|SpawnAIFromClass "/Game/PushContent/Blueprint/BP_RedBuff.BP_RedBuff_C" "/Game/PushContent/Blueprint/WildBehavior/BT_MOBAWildCharacter.BT_MOBAWildCharacter" _returnvalue _returnvalue_2 false)
      (Actor|DestroyActor)
      (elif (Utilities|Enum|Equal(Enum) _returnvalue_3 "Nash")
        (AI|SpawnAIFromClass "/Game/PushContent/Blueprint/BP_Dragon.BP_Dragon_C" "/Game/PushContent/Blueprint/WildBehavior/BT_MOBAWildCharacter.BT_MOBAWildCharacter" _returnvalue _returnvalue_2 false)
        (Actor|DestroyActor)))))

(fn ConstructionScript)