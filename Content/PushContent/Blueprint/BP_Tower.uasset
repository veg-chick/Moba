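; MOBA tower Blueprint that drives its health bar widget and can leave a ruin behind.
; Each Tick, for the local player controller, it pushes the Hp ratio to the TowerUI widget.
; It colours the bar once, green or red, by comparing the tower's camp with the controlled MOBABaseCharacter's.
; The SpawnRuin event spawns a vertically squashed BP_Ruin at the tower's location and rotation.
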(event EventBeginPlay)

(event EventSpawnRuin
  (Game|SpawnActorfromClass "/Game/PushContent/Blueprint/BP_Ruin.BP_Ruin_C" (Math|Transform|MakeTransform (Transformation|GetActorLocation) (Transformation|GetActorRotation) "1,1,0.400000") "AlwaysSpawn" 0 0))

(event EventTick
  (params (DeltaSeconds :type Float%20%28single-precision%29))
  (bind _returnvalue (Game|GetPlayerController 0))
  (bind _astower_ui (Utilities|Casting|CastToTowerUI (UserInterface|GetUserWidgetObject (Variables|Default|GetHp))))
  (Utilities|IsValid _returnvalue
    (:Is%20Valid
      (if (Pawn|IsLocalPlayerController _returnvalue)
        (Utilities|FlowControl|Sequence
          (:then_0
            (bind _returnvalue_2 (Class|MOBABaseCharacter|GetHp))
            (bind _returnvalue_3 (Class|MOBABaseCharacter|GetMaxHp))
            (Variables|/Game/PushContent/HUD/MOBAUI/TowerUI.TowerUI_C|SetHp _astower_ui (/ _returnvalue_2 _returnvalue_3)))
          (:then_1
            (if (not (Variables|Default|GetIsSet))
              (bind _asmobabase_character (Utilities|Casting|CastToMOBABaseCharacter (Pawn|GetControlledPawn _returnvalue)))
              (bind _returnvalue_4 (Class|MOBABaseCharacter|GetCamp))
              (bind _returnvalue_5 (Class|MOBABaseCharacter|GetCamp _asmobabase_character))
              (if (Utilities|Enum|Equal(Enum) _returnvalue_5 _returnvalue_4)
                (Variables|/Game/PushContent/HUD/MOBAUI/TowerUI.TowerUI_C|SetColor _astower_ui (Variables|Default|GetGreen))
                (else
                  (Variables|/Game/PushContent/HUD/MOBAUI/TowerUI.TowerUI_C|SetColor _astower_ui (Variables|Default|GetRed))))
              (Variables|Default|SetIsSet true))))))))

(fn ConstructionScript)