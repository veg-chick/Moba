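; MOBA game mode Blueprint that spawns lane soldiers at the crystals through its SpawnNewSoldier event.
; The event loops over every BP_Crystal and uses the soldier type index to spawn a melee, caster or siege AI pawn at a fixed offset from it, running BT_MOBASoliderCharacter.
; Each soldier inherits the crystal's camp and gets the soldier road matching the crystal's top, mid or down road.
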(event EventBeginPlay)

(event EventSpawnNewSoldier
  (params (SolderType :type Integer))
  (bind _outactors (Actor|GetAllActorsOfClass "/Game/PushContent/Blueprint/BP_Crystal.BP_Crystal_C"))
  (for _array_element _outactors
    (bind _returnvalue (Class|MOBABaseActor|GetCamp _array_element))
    (bind _returnvalue_2 (Class|MOBACrystalActor|GetRoad _array_element))
    (switch int SolderType
      (:0
        (bind _returnvalue_3 (AI|SpawnAIFromClass "/Game/PushContent/Blueprint/Melee_Soldier.Melee_Soldier_C" "/Game/PushContent/Blueprint/SoldierBehavior/BT_MOBASoliderCharacter.BT_MOBASoliderCharacter" (+ (Transformation|GetActorLocation _array_element) "500.000000,500.000000,100.000000") (Transformation|GetActorRotation _array_element) false))
        (bind _asbp_soldier (Utilities|Casting|CastToBP_Soldier _returnvalue_3))
        (Class|MOBASoldierCharacter|ApplyCamp _asbp_soldier _returnvalue)
        (switch Utilities|FlowControl|Switch|SwitchonCrystalRoad _returnvalue_2
          (:crystalTop
            (Class|MOBASoldierCharacter|ApplyRoad _asbp_soldier "soldierTop"))
          (:crystalMid
            (Class|MOBASoldierCharacter|ApplyRoad _asbp_soldier "soldierMid"))
          (:crystalDown
            (Class|MOBASoldierCharacter|ApplyRoad _asbp_soldier "soldierDown"))))
      (:1
        (bind _returnvalue_4 (AI|SpawnAIFromClass "/Game/PushContent/Blueprint/Caster_Soldier.Caster_Soldier_C" "/Game/PushContent/Blueprint/SoldierBehavior/BT_MOBASoliderCharacter.BT_MOBASoliderCharacter" (+ (Transformation|GetActorLocation _array_element) "500.000000,500.000000,100.000000") (Transformation|GetActorRotation _array_element) false))
        (bind _asbp_soldier_2 (Utilities|Casting|CastToBP_Soldier _returnvalue_4))
        (Class|MOBASoldierCharacter|ApplyCamp _asbp_soldier_2 _returnvalue)
        (switch Utilities|FlowControl|Switch|SwitchonCrystalRoad _returnvalue_2
          (:crystalTop
            (Class|MOBASoldierCharacter|ApplyRoad _asbp_soldier_2 "soldierTop"))
          (:crystalMid
            (Class|MOBASoldierCharacter|ApplyRoad _asbp_soldier_2 "soldierMid"))
          (:crystalDown
            (Class|MOBASoldierCharacter|ApplyRoad _asbp_soldier_2 "soldierDown"))))
      (:2
        (bind _returnvalue_5 (AI|SpawnAIFromClass "/Game/PushContent/Blueprint/Siege_Minion.Siege_Minion_C" "/Game/PushContent/Blueprint/SoldierBehavior/BT_MOBASoliderCharacter.BT_MOBASoliderCharacter" (+ (Transformation|GetActorLocation _array_element) "500.000000,500.000000,100.000000") (Transformation|GetActorRotation _array_element) false))
        (bind _asbp_soldier_3 (Utilities|Casting|CastToBP_Soldier _returnvalue_5))
        (Class|MOBASoldierCharacter|ApplyCamp _asbp_soldier_3 _returnvalue)
        (switch Utilities|FlowControl|Switch|SwitchonCrystalRoad _returnvalue_2
          (:crystalTop
            (Class|MOBASoldierCharacter|ApplyRoad _asbp_soldier_3 "soldierTop"))
          (:crystalMid
            (Class|MOBASoldierCharacter|ApplyRoad _asbp_soldier_3 "soldierMid"))
          (:crystalDown
            (Class|MOBASoldierCharacter|ApplyRoad _asbp_soldier_3 "soldierDown")))))))

(fn ConstructionScript)