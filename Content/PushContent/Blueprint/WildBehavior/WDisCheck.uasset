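; Behavior tree node that leashes wild MOBA creatures to their birth place by checking how far they have strayed.
; On tick it caches the owning BP_MOBAWild_Con controller, then measures the 2D distance from its pawn to the BirthPlace blackboard vector.
; It sets the IsGoingBack blackboard flag to true when that distance exceeds MaxDistance, and to false otherwise.
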(event EventTick
  (params (OwnerActor :type Actor%20Object%20Reference) (DeltaSeconds :type Float%20%28single-precision%29))
  (if (!= (Variables|Default|GetMOBAWild_Con_Ref) 0)
    _
    (else
      (bind _asbp_mobawild_con (Utilities|Casting|CastToBP_MOBAWild_Con OwnerActor))
      (bind _output_get (Variables|Default|SetMOBAWild_Con_Ref _asbp_mobawild_con))))
  (bind _output_get_2 (Variables|Default|SetStartLocation (Class|BTFunctionLibrary|GetBlackboardValueasVector (Variables|Default|GetBirthPlace))))
  (Class|BTFunctionLibrary|SetBlackboardValueasBool (Variables|Default|GetIsGoingBack) (not (<= (Math|Vector|Distance2D(Vector) _output_get_2 (Transformation|GetActorLocation (Pawn|GetControlledPawn _output_get))) (Variables|Default|GetMaxDistance)))))