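; WInit is a behavior tree task that initializes a MOBA wild unit's AI blackboard, recording where it starts.
; On execute it casts the owner to BP_MOBAWild_Con, caching the reference for later runs.
; It stores the controlled pawn's current location as BirthLocation, sets Isinit to true and finishes successfully.
; A failed cast stops execution without finishing the task.
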(event EventReceiveExecute
  (params (OwnerActor :type Actor%20Object%20Reference))
  (if (!= (Variables|Default|GetMOBAWild_Con_Ref) 0)
    _
    (else
      (bind _asbp_mobawild_con (Utilities|Casting|CastToBP_MOBAWild_Con OwnerActor))
      (bind _output_get (Variables|Default|SetMOBAWild_Con_Ref _asbp_mobawild_con))))
  (AI|BehaviorTree|SetBlackboardValueasVector (Variables|Default|GetBirthLocation) (Transformation|GetActorLocation (Pawn|GetControlledPawn _output_get)))
  (Class|BTFunctionLibrary|SetBlackboardValueasBool (Variables|Default|GetIsinit) true)
  (AI|BehaviorTree|FinishExecute true))