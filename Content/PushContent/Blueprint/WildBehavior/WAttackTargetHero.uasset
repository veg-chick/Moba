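; Behavior tree task that makes a MOBA wild creature attack the hero stored in its TargetHero blackboard value.
; On execute it caches the wild AI controller, then gets the controlled creature and the target hero.
; It snaps the creature's rotation to face the hero, triggers a single attack and immediately finishes with success.
; A failed cast stops the graph without calling FinishExecute.
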(event EventReceiveExecute
  (params (OwnerActor :type Actor%20Object%20Reference))
  (if (!= (Variables|Default|GetMOBAWild_Con_Ref) 0)
    _
    (else
      (bind _asbp_mobawild_con (Utilities|Casting|CastToBP_MOBAWild_Con OwnerActor))
      (bind _output_get (Variables|Default|SetMOBAWild_Con_Ref _asbp_mobawild_con))))
  (bind _asmobawild_character (Utilities|Casting|CastToMOBAWildCharacter (Pawn|GetControlledPawn _output_get)))
  (bind _asmobahero_character (Utilities|Casting|CastToMOBAHeroCharacter (Class|BTFunctionLibrary|GetBlackboardValueasObject (Variables|Default|GetTargetHero))))
  (Transformation|SetActorRotation _asmobawild_character (Math|Conversions|RotationFromXVector (Math|Vector|Normalize (- (Transformation|GetActorLocation _asmobahero_character) (Transformation|GetActorLocation _asmobawild_character)))))
  (Class|MOBAWildCharacter|AttacktoCharacterOnce _asmobawild_character _asmobahero_character)
  (AI|BehaviorTree|FinishExecute true))