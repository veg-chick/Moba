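; Behavior tree task that moves a MOBA wild character toward the hero stored in the TargetHero blackboard value.
; On execute it caches the wild AI controller from the owner on first use, then reads the hero and the controlled pawn.
; It issues a move to the hero's current location using attack range as acceptance radius, then finishes successfully without waiting for arrival.
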(event EventReceiveExecute
  (params (OwnerActor :type Actor%20Object%20Reference))
  (if (!= (Variables|Default|GetMOBAWild_Con_Ref) 0)
    _
    (else
      (bind _asbp_mobawild_con (Utilities|Casting|CastToBP_MOBAWild_Con OwnerActor))
      (bind _output_get (Variables|Default|SetMOBAWild_Con_Ref _asbp_mobawild_con))))
  (bind _asmobahero_character (Utilities|Casting|CastToMOBAHeroCharacter (Class|BTFunctionLibrary|GetBlackboardValueasObject (Variables|Default|GetTargetHero))))
  (bind _asmobawild_character (Utilities|Casting|CastToMOBAWildCharacter (Pawn|GetControlledPawn _output_get)))
  (bind _returnvalue (Class|MOBABaseCharacter|GetAttackRange _asmobawild_character))
  (AI|Navigation|MovetoLocation _output_get (Transformation|GetActorLocation _asmobahero_character) _returnvalue true true false true 0)
  (AI|BehaviorTree|FinishExecute true))