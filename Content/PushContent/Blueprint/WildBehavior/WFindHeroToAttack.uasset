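; Behavior tree task for MOBA wild units that sets the hero to attack from the unit's current attacker.
; On execute it caches the wild AI controller from the owner, then reads the attacker from its controlled MOBAWildCharacter.
; It writes a valid attacker to the HeroToAttack blackboard key, or clears the key otherwise, and finishes successfully.
; A failed cast leaves the task without a finish call.
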(event EventReceiveExecute
  (params (OwnerActor :type Actor%20Object%20Reference))
  (bind _herotoattack (Variables|Default|GetHeroToAttack))
  (if (!= (Variables|Default|GetMOBAWild_Con_Ref) 0)
    _
    (else
      (bind _asbp_mobawild_con (Utilities|Casting|CastToBP_MOBAWild_Con OwnerActor))
      (bind _output_get (Variables|Default|SetMOBAWild_Con_Ref _asbp_mobawild_con))))
  (bind _asmobawild_character (Utilities|Casting|CastToMOBAWildCharacter (Pawn|GetControlledPawn _output_get)))
  (bind _returnvalue (Class|MOBAWildCharacter|GetAttacker _asmobawild_character))
  (if (Utilities|IsValid _returnvalue)
    (Class|BTFunctionLibrary|SetBlackboardValueasObject _herotoattack _returnvalue)
    (else
      (Class|BTFunctionLibrary|SetBlackboardValueasObject _herotoattack)))
  (AI|BehaviorTree|FinishExecute true))