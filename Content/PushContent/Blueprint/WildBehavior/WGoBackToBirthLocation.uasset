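; Behavior tree task that sends a wild MOBA creature back to its birth location.
; Each execution caches the wild controller, issues a move to the BirthLocation blackboard value and finishes successfully without waiting for arrival.
; When the pawn is already within BackDistance in 2D, it also clears IsGoingBack and TargetHero, then calls QuickRecovery on the character.
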(event EventReceiveExecute
  (params (OwnerActor :type Actor%20Object%20Reference))
  (bind _birthlocation (Variables|Default|GetBirthLocation))
  (bind _returnvalue (Class|BTFunctionLibrary|GetBlackboardValueasVector _birthlocation))
  (if (!= (Variables|Default|GetMOBAWild_Con_Ref) 0)
    _
    (else
      (bind _asbp_mobawild_con (Utilities|Casting|CastToBP_MOBAWild_Con OwnerActor))
      (bind _output_get (Variables|Default|SetMOBAWild_Con_Ref _asbp_mobawild_con))))
  (AI|Navigation|MovetoLocation _output_get _returnvalue -1.0 true true false true 0)
  (if (<= (Math|Vector|Distance2D(Vector) _returnvalue (Transformation|GetActorLocation (Pawn|GetControlledPawn (Variables|Default|GetMOBAWild_Con_Ref)))) (Variables|Default|GetBackDistance))
    (Class|BTFunctionLibrary|SetBlackboardValueasBool (Variables|Default|GetIsGoingBack) (not (<= (Math|Vector|Distance2D(Vector) _returnvalue (Transformation|GetActorLocation (Pawn|GetControlledPawn (Variables|Default|GetMOBAWild_Con_Ref)))) (Variables|Default|GetBackDistance))))
    (Class|BTFunctionLibrary|SetBlackboardValueasObject (Variables|Default|GetTargetHero))
    (bind _asmobawild_character (Utilities|Casting|CastToMOBAWildCharacter (Pawn|GetControlledPawn (Variables|Default|GetMOBAWild_Con_Ref))))
    (Class|MOBAWildCharacter|QuickRecovery _asmobawild_character))
  (AI|BehaviorTree|FinishExecute true))