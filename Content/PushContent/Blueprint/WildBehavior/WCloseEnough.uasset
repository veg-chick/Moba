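; A behavior tree decorator for MOBA wild creature AI that tests whether the target hero is close enough to attack.
; It caches the owning BP_MOBAWild_Con controller, then reads the TargetHero blackboard value and the controlled wild character.
; The check passes when their 2D distance is within the wild character's attack range plus both capsule radii, ignoring height differences.
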(fn PerformConditionCheck
  (params (OwnerActor :type Actor%20Object%20Reference))
  (if (!= (Variables|Default|GetMOBAWild_Con_Ref) 0)
    _
    (else
      (bind _asbp_mobawild_con (Utilities|Casting|CastToBP_MOBAWild_Con OwnerActor))
      (bind _output_get (Variables|Default|SetMOBAWild_Con_Ref _asbp_mobawild_con))))
  (bind _asmobahero_character (Utilities|Casting|CastToMOBAHeroCharacter (Class|BTFunctionLibrary|GetBlackboardValueasObject (Variables|Default|GetTargetHero))))
  (bind _asmobawild_character (Utilities|Casting|CastToMOBAWildCharacter (Pawn|GetControlledPawn _output_get)))
  (bind _returnvalue (Class|MOBABaseCharacter|GetAttackRange _asmobawild_character))
  (return (<= (Math|Vector|Distance2D(Vector) (Transformation|GetActorLocation _asmobawild_character) (Transformation|GetActorLocation _asmobahero_character)) (+ (Components|Capsule|GetScaledCapsuleRadius (Variables|/Script/Engine.Character|GetCapsuleComponent _asmobawild_character)) _returnvalue (Components|Capsule|GetScaledCapsuleRadius (Variables|/Script/Engine.Character|GetCapsuleComponent _asmobahero_character))))))