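; BP_Soldier is a MOBA soldier Blueprint that drives its own health bar display through an Hp widget component.
; Every Tick it casts that widget to SoldierUI and sets its Hp to current over max health.
; It then compares its camp with player 0's MOBABaseCharacter camp, coloring the bar green for the same camp and red otherwise.
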(event EventBeginPlay)

(event Collision|EventActorBeginOverlap
  (params (OtherActor :type Actor%20Object%20Reference)))

(event EventTick
  (params (DeltaSeconds :type Float%20%28single-precision%29))
  (Utilities|FlowControl|Sequence
    (:then_0
      (bind _assoldier_ui (Utilities|Casting|CastToSoldierUI (UserInterface|GetUserWidgetObject (Variables|Default|GetHp))))
      (bind _returnvalue (Class|MOBABaseCharacter|GetHp))
      (bind _returnvalue_2 (Class|MOBABaseCharacter|GetMaxHp))
      (Variables|/Game/PushContent/HUD/MOBAUI/SoldierUI.SoldierUI_C|SetHp _assoldier_ui (/ _returnvalue _returnvalue_2)))
    (:then_1
      (bind _returnvalue_3 (Class|MOBABaseCharacter|GetCamp))
      (bind _asmobabase_character (Utilities|Casting|CastToMOBABaseCharacter (Game|GetPlayerCharacter 0)))
      (bind _returnvalue_4 (Class|MOBABaseCharacter|GetCamp _asmobabase_character))
      (if (Utilities|Enum|Equal(Enum) _returnvalue_3 _returnvalue_4)
        (Variables|/Game/PushContent/HUD/MOBAUI/SoldierUI.SoldierUI_C|SetColor _assoldier_ui (Variables|Default|GetGreen))
        (else
          (Variables|/Game/PushContent/HUD/MOBAUI/SoldierUI.SoldierUI_C|SetColor _assoldier_ui (Variables|Default|GetRed)))))))

(fn ConstructionScript)