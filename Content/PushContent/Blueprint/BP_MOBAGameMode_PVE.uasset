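; PVE MOBA game mode that spawns players as Blue-camp heroes and provides events to spawn lane soldiers and jungle monsters.
; ChoosePlayerStart hands out each PlayerStart once, removing it from the list cached at BeginPlay.
; SpawnNewSoldier spawns a melee, caster or siege soldier at every crystal, applying level, camp and lane.
; Dragons and buff monsters spawn at hardcoded mirrored positions; the bound kill handlers are empty.
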(event Custom|OnActorKilled_事件_0
  (params (VictimActor :type MOBA%20Base%20Actor%20Object%20Reference) (KillerCharacter :type MOBA%20Base%20Character%20Object%20Reference)))

(event Custom|OnCharacterKilled_事件_0
  (params (VictimCharacter :type MOBA%20Base%20Character%20Object%20Reference) (KillerCharacter :type MOBA%20Base%20Character%20Object%20Reference)))

(event EventBeginPlay
  (Utilities|FlowControl|Sequence
    (:then_0
      (EventDispatchers|AssignOnActorKilled (delegate Custom|OnActorKilled_事件_0))
      (EventDispatchers|AssignOnCharacterKilled (delegate Custom|OnCharacterKilled_事件_0)))
    (:then_1
      (bind _outactors (Actor|GetAllActorsOfClass "/Script/Engine.PlayerStart"))
      (Variables|Default|SetPlayerStarts _outactors))))

(event EventSpawnNewSoldier
  (params (SolderType :type Integer))
  (bind _outactors (Actor|GetAllActorsOfClass "/Game/PushContent/Blueprint/BP_Crystal.BP_Crystal_C"))
  (for _array_element _outactors
    (bind _returnvalue (Class|MOBABaseActor|GetCamp _array_element))
    (bind _returnvalue_2 (Class|MOBACrystalActor|GetRoad _array_element))
    (switch int SolderType
      (:0
        (bind _returnvalue_3 (AI|SpawnAIFromClass "/Game/PushContent/Blueprint/Melee_Soldier.Melee_Soldier_C" 0 (Transformation|GetSocketLocation (Variables|/Game/PushContent/Blueprint/BP_Crystal.BP_Crystal_C|GetSoldierSpawn _array_element) "None") (Transformation|GetActorRotation _array_element) false))
        (bind _asbp_soldier (Utilities|Casting|CastToBP_Soldier _returnvalue_3))
        (Class|MOBABaseCharacter|SetLevel _asbp_soldier (Math|Conversions|ToFloat(Integer) (Variables|Default|GetSoldierLevel)))
        (Class|MOBASoldierCharacter|ApplyCamp _asbp_soldier _returnvalue)
        (switch Utilities|FlowControl|Switch|SwitchonCrystalRoad _returnvalue_2
          (:crystalTop
            (Class|MOBASoldierCharacter|ApplyRoad _asbp_soldier "soldierTop"))
          (:crystalMid
            (Class|MOBASoldierCharacter|ApplyRoad _asbp_soldier "soldierMid"))
          (:crystalDown
            (Class|MOBASoldierCharacter|ApplyRoad _asbp_soldier "soldierDown"))))
      (:1
        (bind _returnvalue_4 (AI|SpawnAIFromClass "/Game/PushContent/Blueprint/Caster_Soldier.Caster_Soldier_C" 0 (Transformation|GetSocketLocation (Variables|/Game/PushContent/Blueprint/BP_Crystal.BP_Crystal_C|GetSoldierSpawn _array_element) "None") (Transformation|GetActorRotation _array_element) false))
        (bind _asbp_soldier_2 (Utilities|Casting|CastToBP_Soldier _returnvalue_4))
        (Class|MOBASoldierCharacter|SetSoldierLevel _asbp_soldier_2 (Math|Conversions|ToFloat(Integer) (Variables|Default|GetSoldierLevel)))
        (Class|MOBASoldierCharacter|ApplyCamp _asbp_soldier_2 _returnvalue)
        (switch Utilities|FlowControl|Switch|SwitchonCrystalRoad _returnvalue_2
          (:crystalTop
            (Class|MOBASoldierCharacter|ApplyRoad _asbp_soldier_2 "soldierTop"))
          (:crystalMid
            (Class|MOBASoldierCharacter|ApplyRoad _asbp_soldier_2 "soldierMid"))
          (:crystalDown
            (Class|MOBASoldierCharacter|ApplyRoad _asbp_soldier_2 "soldierDown"))))
      (:2
        (bind _returnvalue_5 (AI|SpawnAIFromClass "/Game/PushContent/Blueprint/Siege_Minion.Siege_Minion_C" 0 (Transformation|GetSocketLocation (Variables|/Game/PushContent/Blueprint/BP_Crystal.BP_Crystal_C|GetSoldierSpawn _array_element) "None") (Transformation|GetActorRotation _array_element) false))
        (bind _asbp_soldier_3 (Utilities|Casting|CastToBP_Soldier _returnvalue_5))
        (Class|MOBABaseCharacter|SetLevel _asbp_soldier_3 (Math|Conversions|ToFloat(Integer) (Variables|Default|GetSoldierLevel)))
        (Class|MOBASoldierCharacter|ApplyCamp _asbp_soldier_3 _returnvalue)
        (switch Utilities|FlowControl|Switch|SwitchonCrystalRoad _returnvalue_2
          (:crystalTop
            (Class|MOBASoldierCharacter|ApplyRoad _asbp_soldier_3 "soldierTop"))
          (:crystalMid
            (Class|MOBASoldierCharacter|ApplyRoad _asbp_soldier_3 "soldierMid"))
          (:crystalDown
            (Class|MOBASoldierCharacter|ApplyRoad _asbp_soldier_3 "soldierDown")))))))

(event EventSpawnStartWild
  (AI|SpawnAIFromClass "/Game/PushContent/Blueprint/BP_BlueBuff.BP_BlueBuff_C" "/Game/PushContent/Blueprint/WildBehavior/BT_MOBAWildCharacter.BT_MOBAWildCharacter" "-2400.000000,6220.000000,0.000000" "0,-90.000000, 0" false)
  (AI|SpawnAIFromClass "/Game/PushContent/Blueprint/BP_BlueBuff.BP_BlueBuff_C" "/Game/PushContent/Blueprint/WildBehavior/BT_MOBAWildCharacter.BT_MOBAWildCharacter" "2400.000000,-6220.000000,0.000000" "0,90.000000, 0" false)
  (AI|SpawnAIFromClass "/Game/PushContent/Blueprint/BP_RedBuff.BP_RedBuff_C" "/Game/PushContent/Blueprint/WildBehavior/BT_MOBAWildCharacter.BT_MOBAWildCharacter" "-6690.000000,1620.000000,0.000000" "0, 0, 0" false)
  (AI|SpawnAIFromClass "/Game/PushContent/Blueprint/BP_RedBuff.BP_RedBuff_C" "/Game/PushContent/Blueprint/WildBehavior/BT_MOBAWildCharacter.BT_MOBAWildCharacter" "6690.000000,-1620.000000,0.000000" "0,180.000000, 0" false))

(event EventSpawnStartDragon
  (AI|SpawnAIFromClass "/Game/PushContent/Blueprint/BP_Dragon.BP_Dragon_C" "/Game/PushContent/Blueprint/WildBehavior/BT_MOBAWildCharacter.BT_MOBAWildCharacter" "-4800.000000,3400.000000,0.000000" "0,135.000000, 0" false)
  (AI|SpawnAIFromClass "/Game/PushContent/Blueprint/BP_Dragon.BP_Dragon_C" "/Game/PushContent/Blueprint/WildBehavior/BT_MOBAWildCharacter.BT_MOBAWildCharacter" "4800.000000,-3400.000000,0.000000" "0,-45.000000, 0" false))

(fn ConstructionScript)

(fn ChoosePlayerStart
  (params (Player :type Controller%20Object%20Reference))
  (bind _playerstarts (Variables|Default|GetPlayerStarts))
  (for _array_element _playerstarts
    (bind _output_get (Variables|Default|SetPlayerStart _array_element))
    (Utilities|Array|RemoveItem _playerstarts _array_element)
    (return _output_get)))

(fn SpawnDefaultPawnatTransform
  (params (NewPlayer :type Controller%20Object%20Reference) (SpawnTransform :type Transform%20%28by%20ref%29))
  (bind _returnvalue (Game|SpawnActorfromClass "/Game/PushContent/Blueprint/BP_MOBAHeroCharacter.BP_MOBAHeroCharacter_C" SpawnTransform "Undefined" 0 0))
  (Class|MOBABaseCharacter|SetCamp _returnvalue "blue")
  (return _returnvalue))