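; Behavior tree task for MOBA towers that picks an enemy hero to attack for harming the tower's allied heroes.
; It scans all hero characters for attackable opposing-camp heroes within 2D attack range that the tower reports as attacking its heroes, keeping the nearest.
; It writes that hero to the HeroToAttack blackboard key and succeeds, or clears the key and fails.
; TargetHero is not reset between executions.
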(event EventReceiveExecute
  (params (OwnerActor :type Actor%20Object%20Reference))
  (bind _herotoattack (Variables|Default|GetHeroToAttack))
  (if (!= (Variables|Default|GetMOBATowerCon_Ref) 0)
    _
    (else
      (bind _asbp_mobatower_con (Utilities|Casting|CastToBP_MOBATower_Con OwnerActor))
      (bind _output_get (Variables|Default|SetMOBATowerCon_Ref _asbp_mobatower_con))))
  (bind _asmobatower_character (Utilities|Casting|CastToMOBATowerCharacter (Pawn|GetControlledPawn _output_get)))
  (bind _returnvalue (Class|MOBABaseCharacter|GetCamp _asmobatower_character))
  (Variables|Default|SetMyCamp _returnvalue)
  (Variables|Default|SetMyLocation (Transformation|GetActorLocation (Pawn|GetControlledPawn _output_get)))
  (Variables|Default|SetMinDistance 99999.0)
  (bind _outactors (Actor|GetAllActorsOfClass "/Script/AMOBAProject.MOBAHeroCharacter"))
  (bind _output_get_2 (Variables|Default|SetAllHeroes _outactors))
  (for _array_element _output_get_2
    (bind _returnvalue_2 (Class|MOBABaseCharacter|GetCamp _array_element))
    (bind _returnvalue_3 (Class|MOBABaseCharacter|GetbCanbeAttacked _array_element))
    (bind _returnvalue_4 (Class|MOBATowerCharacter|IsEnemyHeroAttackingMyHero _asmobatower_character _array_element))
    (bind _returnvalue_5 (Class|MOBABaseCharacter|GetAttackRange _asmobatower_character))
    (if (Math|Boolean|ANDBoolean (<= (Math|Vector|Distance2D(Vector) (Transformation|GetActorLocation _array_element) (Variables|Default|GetMyLocation)) _returnvalue_5) (Utilities|Enum|NotEqual(Enum) _returnvalue_2 (Variables|Default|GetMyCamp)) _returnvalue_3 _returnvalue_4)
      (if (< (Math|Vector|Distance2D(Vector) (Transformation|GetActorLocation _array_element) (Variables|Default|GetMyLocation)) (Variables|Default|GetMinDistance))
        (Variables|Default|SetMinDistance (Math|Vector|Distance2D(Vector) (Transformation|GetActorLocation _array_element) (Variables|Default|GetMyLocation)))
        (Variables|Default|SetTargetHero _array_element))))
  (if (Utilities|IsValid (Variables|Default|GetTargetHero))
    (Class|BTFunctionLibrary|SetBlackboardValueasObject _herotoattack (Variables|Default|GetTargetHero))
    (AI|BehaviorTree|FinishExecute true)
    (else
      (Class|BTFunctionLibrary|SetBlackboardValueasObject _herotoattack)
      (AI|BehaviorTree|FinishExecute false))))