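; Behavior tree task that makes a MOBA tower attack a target soldier once.
; It caches the owning tower AI controller on first execution, then reads the soldier from the TargetSoldier blackboard key.
; It calls AttackToCharacterOnce on the controlled tower pawn and finishes successfully right away.
; A failed cast stops execution without calling FinishExecute.
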(event EventReceiveExecute
  (params (OwnerActor :type Actor%20Object%20Reference))
  (if (!= (Variables|Default|GetMOBATowerCon_Ref) 0)
    _
    (else
      (bind _asbp_mobatower_con (Utilities|Casting|CastToBP_MOBATower_Con OwnerActor))
      (bind _output_get (Variables|Default|SetMOBATowerCon_Ref _asbp_mobatower_con))))
  (bind _asmobasoldier_character (Utilities|Casting|CastToMOBASoldierCharacter (Class|BTFunctionLibrary|GetBlackboardValueasObject (Variables|Default|GetTargetSoldier))))
  (bind _asmobatower_character (Utilities|Casting|CastToMOBATowerCharacter (Pawn|GetControlledPawn _output_get)))
  (Class|MOBATowerCharacter|AttacktoCharacterOnce _asmobatower_character _asmobasoldier_character)
  (AI|BehaviorTree|FinishExecute true))