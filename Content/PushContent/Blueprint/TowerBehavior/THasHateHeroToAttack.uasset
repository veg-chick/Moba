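; Behavior tree condition for MOBA tower AI that checks whether the tower has a hated hero it can still attack.
; It caches the tower controller from the owner, then reads the TargetHateHero blackboard key.
; It passes when that hero has nonzero HP and is within the tower pawn's attack range, measured in 2D.
; A valid target that fails either test is cleared from the blackboard.
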(fn PerformConditionCheck
  (params (OwnerActor :type Actor%20Object%20Reference))
  (bind _targethatehero (Variables|Default|GetTargetHateHero))
  (bind _returnvalue (Class|BTFunctionLibrary|GetBlackboardValueasObject _targethatehero))
  (if (!= (Variables|Default|GetMOBATowerCon_Ref) 0)
    _
    (else
      (bind _asbp_mobatower_con (Utilities|Casting|CastToBP_MOBATower_Con OwnerActor))
      (bind _output_get (Variables|Default|SetMOBATowerCon_Ref _asbp_mobatower_con))))
  (if (Utilities|IsValid _returnvalue)
    (bind _asmobabase_character (Utilities|Casting|CastToMOBABaseCharacter _returnvalue))
    (bind _returnvalue_2 (Class|MOBABaseCharacter|GetHp _asmobabase_character))
    (bind _asmobabase_character_2 (Utilities|Casting|CastToMOBABaseCharacter (Pawn|GetControlledPawn _output_get)))
    (bind _returnvalue_3 (Class|MOBABaseCharacter|GetAttackRange _asmobabase_character_2))
    (if (and (!= _returnvalue_2 0.0) (<= (Math|Vector|Distance2D(Vector) (Transformation|GetActorLocation _asmobabase_character) (Transformation|GetActorLocation (Pawn|GetControlledPawn _output_get))) _returnvalue_3))
      (return true)
      (else
        (Class|BTFunctionLibrary|SetBlackboardValueasObject (Variables|Default|GetTargetHateHero))
        (return false)))
    (else
      (return false))))